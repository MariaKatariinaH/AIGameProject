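; Player hero character that moves, jumps, aims and shoots, counts collected candies, and shows a health bar widget.
; While aiming, holding Fire repeats camera-based line traces on a looping timer, spawning muzzle effects and applying point damage to BP_MyEnemy.
; An equip event switches whether rotation follows controller yaw, toggled by a debug key.
; Lethal point damage ragdolls the mesh with a hit impulse, then reloads the level after a delay.
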(event Custom|Equip%20/%20Holster
  (params (Equip? :type Boolean))
  ;[1 1 1] Equip
  ;;[1 1 1] When weapon is equipped, character rotation follows mouse
  (if Equip?
    (Variables|Default|SetbUseControllerRotationYaw true)
    (else
      (Variables|Default|SetbUseControllerRotationYaw false))))

(event Custom|Fire
  (bind _camera (Variables|Default|GetCamera))
  (bind _returnvalue (Transformation|GetWorldLocation _camera))
  ;[1 1 1] When timer is finished, shoot line trace towards where camera is pointing.
  (if (not (Variables|Default|GetIsDead))
    (bind _outhit (Collision|LineTraceByChannel _returnvalue (+ _returnvalue (* (Math|Vector|GetForwardVector _camera) 1e+06)) "TraceTypeQuery1" false 0 "ForDuration"))
    (Effects|SpawnEmitteratLocation "/Game/StarterContent/Particles/P_Explosion.P_Explosion" (Transformation|GetWorldLocation (Variables|Default|GetBarrelLocation)) "0, 0, 0" "0.100000,0.100000,0.100000")
    (bind _asbp_my_enemy (Utilities|Casting|CastToBP_MyEnemy (.HitActor (Collision|BreakHitResult _outhit))))
    (Game|Damage|ApplyPointDamage _asbp_my_enemy 1e+02 (.Normal (Collision|BreakHitResult _outhit)) _outhit 0 self)))

(event EventBeginPlay
  (bind _returnvalue (UserInterface|CreateWidget "/Game/UI/WB_PlayerHealthBar.WB_PlayerHealthBar_C"))
  (UserInterface|Viewport|AddtoViewport _returnvalue 0))

(event Collision|EventActorBeginOverlap
  (params (OtherActor :type Actor%20Object%20Reference))
  (|CallParentFunction OtherActor) ; This node is disabled and will not be called.\nDrag off pins to build functionality.
)

(event Game|Damage|EventPointDamage
  (params (Damage :type Float%20%28single-precision%29) (DamageType :type Damage%20Type%20Object%20Reference) (HitLocation :type Vector :default "0, 0, 0") (HitNormal :type Vector :default "0, 0, 0") (HitComponent :type Primitive%20Component%20Object%20Reference) (BoneName :type Name :default "None") (ShotFromDirection :type Vector :default "0, 0, 0") (InstigatedBy :type Controller%20Object%20Reference) (DamageCauser :type Actor%20Object%20Reference) (HitInfo :type Hit%20Result%20Structure%20%28by%20ref%29))
  (bind _output_get (Variables|Default|SetHealth (- (Variables|Default|GetHealth) Damage)))
  (if (<= _output_get 0.0)
    (Variables|Default|SetIsDead true)
    (Collision|SetCollisionEnabled (Variables|Character|GetMesh) "QueryAndPhysics")
    (Collision|SetCollisionEnabled (Variables|Default|GetCapsuleComponent) "NoCollision")
    (Physics|SetSimulatePhysics (Variables|Character|GetMesh) true)
    (Physics|AddImpulseatLocation (Variables|Character|GetMesh) (* HitNormal 6e+04 -1) HitLocation BoneName)
    (Utilities|FlowControl|Delay 5.0)
    (bind _returnvalue (Game|GetCurrentLevelName true))
    (Game|OpenLevel(byName) (Utilities|String|StringToName _returnvalue))))

(event Input|ActionEvents|InputActionAim
  (params (Key :type Key%20Structure :default "None"))
  ;[1 1 1] Aiming
  (:Pressed
    (Variables|Default|SetAiming true))
  (:Released
    (Variables|Default|SetAiming false)))

(event Input|ActionEvents|InputActionFire
  (params (Key :type Key%20Structure :default "None"))
  (bind _isdead (Variables|Default|GetIsDead))
  (bind _camera (Variables|Default|GetCamera))
  (bind _returnvalue (Transformation|GetWorldLocation _camera))
  ;[1 1 1] When pressing mouse, start timer which does Line Trace checking. Only activate if aiming (holding right mouse)
  (:Pressed
    (if (not _isdead)
      (if (Variables|Default|GetAiming)
        (bind _returnvalue_2 (Utilities|Time|SetTimerbyEvent (delegate Custom|Fire) 0.1 true))
        (Variables|Default|SetFireTimer _returnvalue_2)
        ;[1 1 1] When timer is finished, shoot line trace towards where camera is pointing.
        (bind _outhit (Collision|LineTraceByChannel _returnvalue (+ _returnvalue (* (Math|Vector|GetForwardVector _camera) 1e+06)) "TraceTypeQuery1" false 0 "ForDuration"))
        (Effects|SpawnEmitteratLocation "/Game/StarterContent/Particles/P_Explosion.P_Explosion" (Transformation|GetWorldLocation (Variables|Default|GetBarrelLocation)) "0, 0, 0" "0.100000,0.100000,0.100000")
        (bind _asbp_my_enemy (Utilities|Casting|CastToBP_MyEnemy (.HitActor (Collision|BreakHitResult _outhit))))
        (Game|Damage|ApplyPointDamage _asbp_my_enemy 1e+02 (.Normal (Collision|BreakHitResult _outhit)) _outhit 0 self))))
  (:Released
    (if (not _isdead)
      (Utilities|Time|ClearandInvalidateTimerbyHandle (Variables|Default|GetFireTimer)))))

(event Input|ActionEvents|InputActionJump
  (params (Key :type Key%20Structure :default "None"))
  (:Pressed
    (Character|Jump)
    (Components|Animation|PlayAnimation (Variables|Character|GetMesh) "/Game/Characters/Biker/Animations/Jump_Montage.Jump_Montage" false)
    (Utilities|FlowControl|Delay 1.5)
    (Components|Animation|SetAnimationMode (Variables|Character|GetMesh) "AnimationBlueprint" true))
  (:Released
    (Character|StopJumping)))

(event Input|AxisEvents|InputAxisLookRight
  (params (AxisValue :type Float%20%28single-precision%29))
  ;[1 1 1] Move
  (Pawn|Input|AddControllerYawInput AxisValue))

(event Input|AxisEvents|InputAxisLookUp
  (params (AxisValue :type Float%20%28single-precision%29))
  ;[1 1 1] Move
  (Pawn|Input|AddControllerPitchInput (* AxisValue (Math|Float|SelectFloat 1.0 -1.0 (Variables|Default|GetInvert%20pitch)))))

(event Input|AxisEvents|InputAxisMoveForward
  (params (AxisValue :type Float%20%28single-precision%29))
  ;[1 1 1] Move
  (if (not (Variables|Default|GetIsDead))
    (Pawn|Input|AddMovementInput (Math|Vector|GetForwardVector (Transformation|GetActorRotation)) AxisValue false)))

(event Input|AxisEvents|InputAxisMoveRight
  (params (AxisValue :type Float%20%28single-precision%29))
  ;[1 1 1] Move
  (if (not (Variables|Default|GetIsDead))
    (Pawn|Input|AddMovementInput (Math|Vector|GetRightVector (Transformation|GetActorRotation)) AxisValue false)))

(event Input|KeyboardEvents|DebugKeyEnter
  (params (Key :type Key%20Structure :default "None") (ActionValue :type Input%20Action%20Value%20Structure))
  ;[1 1 1] Equip
  (:Pressed
    (Utilities|FlowControl|FlipFlop
      (:A
        (CallFunction|Equip/Holster false))
      (:B
        (CallFunction|Equip/Holster true)))))

(fn ConstructionScript
  (|CallParentFunction))

(fn AddCandy
  (Variables|Default|SetTotalCandies (+ (Variables|Default|GetTotalCandies) 1)))