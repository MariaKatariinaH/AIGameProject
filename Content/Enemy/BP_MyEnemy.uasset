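; Enemy character that fires hitscan shots every second and can be killed by point damage.
; Each shot line-traces from ShootingHelper within a random 10-degree cone, spawns a small muzzle explosion, and applies point damage only if it hits the hero character.
; When health runs out, it stops firing, disables capsule collision and ragdolls the mesh with an impulse at the hit bone.
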(event `self.ReceiveBeginPlay`
  (`self.EnemyFire` :!label _label)
  (`KismetSystemLibrary.Delay` 1.0)
  (goto _label))

(event `EnemyFire`
  (bind _shootinghelper (`self.ShootingHelper`))
  (bind _returnvalue (`SceneComponent.K2_GetComponentLocation` _shootinghelper))
  (if (not (`self.IsDead`))
    (bind _outhit (`KismetSystemLibrary.LineTraceSingle` :`Start` _returnvalue :`End` (+ _returnvalue (* (`KismetMathLibrary.RandomUnitVectorInConeInDegrees` (`KismetMathLibrary.GetForwardVector` (`SceneComponent.K2_GetComponentRotation` _shootinghelper)) 10.0) 10000.0)) :`TraceChannel` "TraceTypeQuery1" :`DrawDebugType` "ForDuration"))
    (`GameplayStatics.SpawnEmitterAtLocation` "/Game/StarterContent/Particles/P_Explosion.P_Explosion" (`SceneComponent.K2_GetComponentLocation` (`self.ShootingHelper`)) (struct) (0.1 0.1 0.1))
    (bind (_bblockinghit _binitialoverlap _time _distance _location _impactpoint _normal _impactnormal _physmat _hitactor) (`GameplayStatics.BreakHitResult` _outhit))
    (bind _asbp_hero_character (cast `/Game/Blueprints/Characters/BP_HeroCharacter` _hitactor))
    (`GameplayStatics.ApplyPointDamage` _asbp_hero_character 25.0 _normal _outhit null self)))

(event `self.ReceivePointDamage`
  (params (Damage :type "Float (single-precision)") (DamageType :type "DamageType Object Reference") (HitLocation :type "Vector Structure") (HitNormal :type "Vector Structure") (HitComponent :type "PrimitiveComponent Object Reference") (BoneName :type Name) (ShotFromDirection :type "Vector Structure") (InstigatedBy :type "Controller Object Reference") (DamageCauser :type "Actor Object Reference") (HitInfo :type "HitResult Structure (by ref)"))
  (bind _output_get (set `self.Health` (- (`self.Health`) Damage)))
  (if (<= _output_get 0.0)
    (set `self.IsDead` true)
    (`PrimitiveComponent.SetCollisionEnabled` (`self.Mesh`) "QueryAndPhysics")
    (`PrimitiveComponent.SetCollisionEnabled` (`self.CapsuleComponent`) "NoCollision")
    (`PrimitiveComponent.SetSimulatePhysics` (`self.Mesh`) true)
    (`PrimitiveComponent.AddImpulseAtLocation` (`self.Mesh`) (* HitNormal 60000.0 -1) HitLocation BoneName)))

(fn `UserConstructionScript`
  (`parent.UserConstructionScript`))